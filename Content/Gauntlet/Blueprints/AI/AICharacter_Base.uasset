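; Base AI character for Gauntlet that tracks health, takes damage and dies with a money drop.
; Any damage lowers CurrentHealth, refreshes the widget health bar and has the game mode display a combo at the character's location.
; At zero health, a DoOnce-guarded OnDeath asks the game mode to drop money, then destroys the actor via a short life span.
; A separate Murder function destroys it immediately.
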(event `self.ReceiveBeginPlay`)

(event `self.ReceiveActorBeginOverlap`
  (params (OtherActor :type "Actor Object Reference")))

(event `self.ReceiveTick`
  (params (DeltaSeconds :type "Float (single-precision)")))

(event `self.ReceiveAnyDamage`
  (params (Damage :type "Float (single-precision)") (DamageType :type "DamageType Object Reference") (InstigatedBy :type "Controller Object Reference") (DamageCauser :type "Actor Object Reference"))
  (bind _output_get (set `self.CurrentHealth` (- (`self.CurrentHealth`) Damage)))
  (`|ExecutionSequence`
    (:`then_0`
      (if (<= _output_get 0.0)
        (`self.OnDeath`)))
    (:`then_1`
      (`self.UpdateHealthBar`)
      (bind _asgame_mode_game (cast `/Game/Gauntlet/Blueprints/GameModeGame` (`GameplayStatics.GetGameMode`)))
      (`/Game/Gauntlet/Blueprints/GameModeGame.DisplayCombo` _asgame_mode_game (`self.K2_GetActorLocation`)))))

(fn `GetHealthPerc`
  (returns (HealthPerc :type "Float (double-precision)"))
  (return (/ (`self.CurrentHealth`) (`self.MaxHealth`))))

(fn `Murder`
  (`self.K2_DestroyActor`))

(fn `OnDeath`
  (`/Engine/EditorBlueprintResources/StandardMacros.DoOnce` false
    (:`Completed`
      (`|ExecutionSequence`
        (:`then_0`
          (bind _asgame_mode_game (cast `/Game/Gauntlet/Blueprints/GameModeGame` (`GameplayStatics.GetGameMode`)))
          (`/Game/Gauntlet/Blueprints/GameModeGame.DropMoney` _asgame_mode_game (`self.K2_GetActorLocation`)))
        (:`then_1`
          (`self.SetLifeSpan` 0.1))))))

(fn `UpdateHealthBar`
  (bind _ashealth_bar (cast `/Game/Gauntlet/Blueprints/HUD/HealthBar` (`WidgetComponent.GetUserWidgetObject` (`self.HealthBar`))))
  (set `/Game/Gauntlet/Blueprints/HUD/HealthBar.HealthPerc` (`self.GetHealthPerc`) _ashealth_bar))

(fn `UserConstructionScript`
  (set `self.CurrentHealth` (`self.MaxHealth`)))