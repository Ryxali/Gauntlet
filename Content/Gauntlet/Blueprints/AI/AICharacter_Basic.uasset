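; Basic AI enemy character for Gauntlet that deals melee damage to the player through a Blade collision component.
; Overlapping a ThirdPersonCharacter stores it as Target and starts Hurt, and ending that overlap clears it.
; Hurt applies damage under the AI controller as instigator, then re-calls itself after a delay while the target stays valid, using a Lock flag to prevent stacked damage loops.
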(event `self.ReceiveBeginPlay`)

(event `self.ReceiveActorBeginOverlap`
  (params (OtherActor :type "Actor Object Reference")))

(event `self.ReceiveTick`
  (params (DeltaSeconds :type "Float (single-precision)")))

(event `self.Blade.OnComponentBeginOverlap`
  (params (OtherActor :type "Actor Object Reference") (OtherComp :type "PrimitiveComponent Object Reference") (OtherBodyIndex :type Integer) (bFromSweep :type Boolean) (SweepResult :type "HitResult Structure (by ref)"))
  (if (== (`GameplayStatics.GetObjectClass` OtherActor) "/Game/ThirdPerson/Blueprints/ThirdPersonCharacter.ThirdPersonCharacter_C")
    (set `self.target` OtherActor)
    (`self.Hurt`)))

(event `self.Blade.OnComponentEndOverlap`
  (params (OtherActor :type "Actor Object Reference") (OtherComp :type "PrimitiveComponent Object Reference") (OtherBodyIndex :type Integer))
  (if (== OtherActor (`self.target`))
    (set `self.target` null)))

(event `Hurt`
  (if (not (`self.lock`))
    (set `self.lock` true)
    (bind _target (`self.target`)
      (:`then`
        (bind _returnvalue (`AIBlueprintHelperLibrary.GetAIController` self))
        (`GameplayStatics.ApplyDamage` _target 5.0 _returnvalue self)
        (`KismetSystemLibrary.Delay` 1.2)
        (set `self.lock` false)
        (`self.Hurt`))
      (:`else`
        (set `self.lock` false)))))

(fn `UserConstructionScript`)