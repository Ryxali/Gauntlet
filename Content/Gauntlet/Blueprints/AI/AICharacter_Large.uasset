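; Large AI character for Gauntlet that fires shockwave projectiles when told to shoot.
; Shootat plays a timeline whose Fire event spawns Projectile_Shockwave just ahead of the actor along its facing, with itself as instigator.
; Firing is false during the timeline and true once it ends, so ShootFinished reports completion through it.
; The turn toward Target is disconnected, so shots ignore the target.
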(event `self.ReceiveBeginPlay`)

(event `self.ReceiveActorBeginOverlap`
  (params (OtherActor :type "Actor Object Reference")))

(event `self.ReceiveTick`
  (params (DeltaSeconds :type "Float (single-precision)")))

(event `/Game/Gauntlet/Blueprints/AI/Shooting.ShootAt`
  (params (Target :type "Actor Object Reference"))
  (set `self.Firing` false)
  (`Timeline|Shoot_Timeline` :!via `PlayFromStart`
    (:`Finished`
      (set `self.Firing` true))
    (:`Fire`
      (`|SpawnActorFromClass` "/Game/Gauntlet/Blueprints/AI/Projectile_Shockwave.Projectile_Shockwave_C" (`KismetMathLibrary.MakeTransform` (+ (`self.K2_GetActorLocation`) (* (`self.GetActorForwardVector`) 16.0)) (`self.K2_GetActorRotation`)) false null self))))

(fn `ShootFinished`
  (returns (Finished :type Boolean))
  (return (`self.Firing`)))

(fn `UserConstructionScript`
  (`parent.UserConstructionScript`))