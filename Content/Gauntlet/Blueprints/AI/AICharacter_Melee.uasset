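; Melee enemy character, a small rock "Pebble" minion with a lunge attack that damages player characters inside its strike sphere.
; Damage triggers sound events, camera shake and a fresnel flash on a dynamic material; death spawns a destructible mesh shattered by radial damage.
; Lunge events (named "Lounge") drive the anim Blueprint and montages, while spawning either plays a burst-out montage or raises it from the navmesh via timeline.
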(event `self.ReceiveAnyDamage`
  (params (Damage :type "Float (single-precision)") (DamageType :type "DamageType Object Reference") (InstigatedBy :type "Controller Object Reference") (DamageCauser :type "Actor Object Reference"))
  (bind _returnvalue (`self.GetTransform`))
  (bind _returnvalue_2 (`KismetMathLibrary.RandomFloatInRange` -100.0 100.0))
  (bind _mesh (`self.Mesh`))
  (bind _returnvalue_3 (`SceneComponent.K2_GetComponentLocation` _mesh))
  (`parent.ReceiveAnyDamage` Damage DamageType InstigatedBy DamageCauser)
  (if (<= (`self.CurrentHealth`) 0.0)
    (`FMODBlueprintStatics.PlayEventAtLocation` "/Game/FMOD/Events/Effect/Enemy/Enemy_Death.Enemy_Death" _returnvalue)
    (`GameplayStatics.PlayWorldCameraShake` "/Game/Gauntlet/Blueprints/HUD/CamShakeSmall2.CamShakeSmall2_C" (`SceneComponent.K2_GetComponentLocation` (`self.Mesh`)) 0.0 10000.0)
    ;[1 1 1] Spawns Destructable mesh on death and destroys it
    (bind _returnvalue_4 (`|SpawnActorFromClass` "/Game/Gauntlet/Blueprints/AI/BP_DestructableSmallMinion.BP_DestructableSmallMinion_C" (`KismetMathLibrary.MakeTransform` _returnvalue_3 (`SceneComponent.K2_GetComponentRotation` _mesh) (1.0 1.0 1.0))))
    (`DestructibleComponent.ApplyRadiusDamage` (`/Game/Gauntlet/Blueprints/AI/BP_DestructableSmallMinion.Destructible` _returnvalue_4) 5.0 (`KismetMathLibrary.MakeVector` (+ _returnvalue_2 (.x _returnvalue_3)) (+ _returnvalue_2 (.y _returnvalue_3)) (+ (.z _returnvalue_3) 100.0)) 300.0 1000.0 false)
    (else
      (`FMODBlueprintStatics.PlayEventAtLocation` "/Game/FMOD/Events/Effect/Enemy/Enemy_Damaged.Enemy_Damaged" _returnvalue)
      (if (== DamageCauser (`Controller.K2_GetPawn` (`GameplayStatics.GetPlayerController` 0)))
        (`GameplayStatics.PlayWorldCameraShake` "/Game/Gauntlet/Blueprints/HUD/CamShakeSmall2.CamShakeSmall2_C" (`SceneComponent.K2_GetComponentLocation` (`self.Mesh`)) 0.0 10000.0)
        ;[1 1 1] Plays fresnel hit effect
        (bind (_direction _newtrack_0) (`Timeline|Timeline_0` :!via `PlayFromStart` :!label _label)
          (:`Update`
            (`MaterialInstanceDynamic.SetScalarParameterValue` (`self.MID`) "FresnelScalar" _newtrack_0)))
        (else
          (goto _label :!via `PlayFromStart`))))))

(event `self.ReceiveBeginPlay`
  (`PrimitiveComponent.SetMaterial` (`self.Mesh`) 0 (`self.MID`)))

(event `self.ReceiveActorBeginOverlap`
  (params (OtherActor :type "Actor Object Reference")))

(event `self.ReceiveTick`
  (params (DeltaSeconds :type "Float (single-precision)")))

(event `/Game/Gauntlet/Blueprints/AI/Lounging.Lounge`
  (params (Target :type "Actor Object Reference"))
  ;[1 1 1] Lounge Related
  (set `self.Lounging` true)
  (bind _aspebble_anim_bp (cast `/Game/Gauntlet/Animation/PebbleAnimBP` (`SkeletalMeshComponent.GetAnimInstance` (`self.Mesh`))))
  (`/Game/Gauntlet/Animation/PebbleAnimBP.StartAttack` _aspebble_anim_bp))

(event `EndLounge`
  ;[1 1 1] Lounge Related
  (set `self.Lounging` false))

(event `Strike`
  ;[1 1 1] Lounge Related
  (for _array_element (`PrimitiveComponent.GetOverlappingActors` (`self.StrikeSphere`) "/Script/Gauntlet.GauntletCharacter")
    (`GameplayStatics.ApplyDamage` _array_element (`self.Damage`) (`self.GetController`) self)))

(event `/Game/Gauntlet/Blueprints/AI/Lounging.LoungeWindup`
  ;[1 1 1] Lounge Related
  (`AnimInstance.Montage_Play` (`SkeletalMeshComponent.GetAnimInstance` (`self.Mesh`)) "/Game/Gauntlet/Animation/Pebble_ChargeWindup_Montage.Pebble_ChargeWindup_Montage" 1.0))

(event `/Game/Gauntlet/Blueprints/AI/Lounging.LoungeCharge`
  (bind _aspebble_anim_bp (cast `/Game/Gauntlet/Animation/PebbleAnimBP` (`SkeletalMeshComponent.GetAnimInstance` (`self.Mesh`))))
  (`/Game/Gauntlet/Animation/PebbleAnimBP.StartCharge` _aspebble_anim_bp))

(event `/Game/Gauntlet/Blueprints/AI/Spawnimated.BeginSpawn`
  (set `self.Spawned` false)
  (switch `/Game/Gauntlet/Blueprints/AI/SpawnAnimationMode` (`self.SpawnAnimationMode`)
    (:`NewEnumerator0`
      (`self.PlayAnimMontage` "/Game/Gauntlet/Animation/Animation_files/BoulderAttack.BoulderAttack"))
    (:`NewEnumerator1`
      (`ActorComponent.SetActive` (`self.CharacterMovement`) false false)
      (set `self.Origin` (+ (`NavigationSystem.ProjectPointToNavigation` (`self.K2_GetActorLocation`)) (* (0.0 0.0 1.0) (`CapsuleComponent.GetScaledCapsuleHalfHeight` (`self.CapsuleComponent`)))))
      (bind (_direction _offset) (`Timeline|Unburrow` :!via `PlayFromStart`)
        (:`Update`
          (`self.K2_SetActorLocation` (+ (* (0.0 0.0 1.0) (* (`CapsuleComponent.GetScaledCapsuleHalfHeight` (`self.CapsuleComponent`)) 2.0 _offset)) (`self.Origin`))))
        (:`Finished`
          (`self.Notify Spawn Finished`)
          (`ActorComponent.SetActive` (`self.CharacterMovement`) true false))))))

(event `Notify Spawn Finished`
  (set `self.Spawned` true))

(fn `LoungeFinished`
  (returns (Finished :type Boolean))
  (return (not (`self.Lounging`))))

(fn `SpawnFinished`
  (returns (Finished :type Boolean))
  (return (`self.Spawned`)))

(fn `UserConstructionScript`
  (`parent.UserConstructionScript`)
  (bind _returnvalue (`KismetMaterialLibrary.CreateDynamicMaterialInstance` "/Game/Gauntlet/Materials/Ma_Char_MiniRock.Ma_Char_MiniRock"))
  (set `self.MID` _returnvalue))