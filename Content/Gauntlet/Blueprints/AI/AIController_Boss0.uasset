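; AI controller for Boss0 that runs its behavior tree and blackboard, held idle until the fight is started.
; BeginPlay sets up the blackboard and runs BTree_Boss0, then immediately stops its logic.
; Start fills the blackboard with the player as Target and an initial AIBossState Phase, then restarts the logic.
; Reset stops the brain again, with "Player Death" as the reason.
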(event `self.ReceiveBeginPlay`
  (bind _blackboardcomponent (`self.UseBlackboard` "/Game/Gauntlet/Blueprints/AI/BBData_Boss0.BBData_Boss0"))
  (set `self.Blackboard` _blackboardcomponent)
  (`self.RunBehaviorTree` "/Game/Gauntlet/Blueprints/AI/BTree_Boss0.BTree_Boss0")
  (`BrainComponent.StopLogic` (`self.BrainComponent`) ""))

(event `self.ReceiveTick`
  (params (DeltaSeconds :type "Float (single-precision)")))

(event `Start`
  (`KismetSystemLibrary.PrintString` "Hello")
  (`self.SetupBlackboard`)
  (`BrainComponent.RestartLogic` (`self.BrainComponent`)))

(event `Reset`
  (`BrainComponent.StopLogic` (`self.BrainComponent`) "Player Death"))

(fn `SetupBlackboard`
  (`BlackboardComponent.SetValueAsObject` (`self.Blackboard`) "Target" (`GameplayStatics.GetPlayerCharacter` 0))
  (`BlackboardComponent.SetValueAsEnum` (`self.Blackboard`) "Phase" (enumliteral `/Game/Gauntlet/Blueprints/AI/AIBossState` "NewEnumerator0")))

(fn `UserConstructionScript`)