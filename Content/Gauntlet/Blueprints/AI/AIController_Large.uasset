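; AI controller for large melee minions in Gauntlet.
; On begin play it sets up the BBData_LargeMinion blackboard, then runs the BTree_LargeMinion behavior tree.
; Blackboard setup sets Target to player 0's controlled pawn and State to an initial melee minion state enum value, leaving all decisions to the tree.
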(event `self.ReceiveBeginPlay`
  (`self.InitializeBlackboard`)
  (`self.RunBehaviorTree` "/Game/Gauntlet/Blueprints/AI/BTree_LargeMinion.BTree_LargeMinion"))

(event `self.ReceiveTick`
  (params (DeltaSeconds :type "Float (single-precision)")))

(fn `InitializeBlackboard`
  (bind (_blackboardcomponent _returnvalue) (`self.UseBlackboard` "/Game/Gauntlet/Blueprints/AI/BBData_LargeMinion.BBData_LargeMinion"))
  (set `self.Blackboard` _blackboardcomponent)
  (if _returnvalue
    (`BlackboardComponent.SetValueAsObject` (`self.Blackboard`) "Target" (`self.K2_GetPawn` (`GameplayStatics.GetPlayerController` 0)))
    (`BlackboardComponent.SetValueAsEnum` (`self.Blackboard`) "State" (enumliteral `/Game/Gauntlet/Blueprints/AI/AIMeleeMinionState` "NewEnumerator0"))))

(fn `UserConstructionScript`)