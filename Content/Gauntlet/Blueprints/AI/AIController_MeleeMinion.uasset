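; AI controller for the melee minion in Gauntlet, which sets up its blackboard and runs the melee minion behavior tree on BeginPlay.
; Blackboard setup stores the first player's pawn as Target and sets State to an initial minion state enum value.
; It also spawns a TargetTracker actor that receives the player pawn as its target and the minion's pawn as its owning actor.
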(event `self.ReceiveBeginPlay`
  (`self.InitializeBlackboard`)
  (`self.RunBehaviorTree` "/Game/Gauntlet/Blueprints/AI/BTree_MeleeMinion.BTree_MeleeMinion"))

(event `self.ReceiveTick`
  (params (DeltaSeconds :type "Float (single-precision)")))

(fn `InitializeBlackboard`
  (bind _returnvalue (`self.K2_GetPawn` (`GameplayStatics.GetPlayerController` 0)))
  (bind (_blackboardcomponent _returnvalue_2) (`self.UseBlackboard` "/Game/Gauntlet/Blueprints/AI/BBData_MeleeMinion.BBData_MeleeMinion"))
  (set `self.Blackboard` _blackboardcomponent)
  (if _returnvalue_2
    (`BlackboardComponent.SetValueAsObject` (`self.Blackboard`) "Target" _returnvalue)
    (`|SpawnActorFromClass` "/Game/Gauntlet/Blueprints/AI/Special/TargetTracker.TargetTracker_C" (`KismetMathLibrary.MakeTransform` (0.0 0.0 0.0)) true null _returnvalue (`self.K2_GetPawn`))
    (`BlackboardComponent.SetValueAsEnum` (`self.Blackboard`) "State" (enumliteral `/Game/Gauntlet/Blueprints/AI/AIMinionState` "NewEnumerator0"))))

(fn `UserConstructionScript`)