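; Boss pawn for the Gauntlet that drops meteor projectiles and summons tracked melee minions.
; A one-shot overlap by the local player creates the boss health HUD and starts AIController_Boss0.
; Damage updates that HUD unless the boss is invulnerable.
; Events expose attacks, minion cleanup and invulnerability, while getters report health and whether shooting or spawning has finished.
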(event `self.ReceiveBeginPlay`
  (set `self.Health` (`self.MaxHealth`)))

(event `self.ReceiveTick`
  (params (DeltaSeconds :type "Float (single-precision)")))

(event `self.ReceiveAnyDamage`
  (params (Damage :type "Float (single-precision)") (DamageType :type "DamageType Object Reference") (InstigatedBy :type "Controller Object Reference") (DamageCauser :type "Actor Object Reference"))
  (if (not (`self.Invulnerable`))
    (bind _output_get (set `self.Health` (- (`self.Health`) Damage)))
    (`/Game/Gauntlet/Blueprints/HUD/BossWidget.SetHpPerc` (`self.BossHUD`) (/ _output_get (`self.MaxHealth`)))))

(event `/Game/Gauntlet/Blueprints/AI/Spawning.KillAllSpawned`
  (`/Game/Gauntlet/Blueprints/AI/AICharacter_Base.Murder` (`self.Spawned`)))

(event `self.ReceiveEndPlay`
  (params (EndPlayReason :type "EEndPlayReason Enum" :default "Destroyed"))
  (`Widget.RemoveFromParent` (`self.BossHUD`)))

(event `self.ReceiveActorBeginOverlap`
  (params (OtherActor :type "Actor Object Reference"))
  (if (`Controller.IsLocalPlayerController` (`self.GetInstigatorController` OtherActor))
    (`/Engine/EditorBlueprintResources/StandardMacros.DoOnce` false :!label _label
      (:`Completed`
        (bind _returnvalue (`|CreateWidget` "/Game/Gauntlet/Blueprints/HUD/BossWidget.BossWidget_C" (`GameplayStatics.GetPlayerController` 0)))
        (bind _output_get (set `self.BossHUD` _returnvalue))
        (`UserWidget.AddToViewport` _output_get 1000)
        (bind _asaicontroller_boss_0 (cast `/Game/Gauntlet/Blueprints/AI/AIController_Boss0` (`self.GetController`)))
        (`/Game/Gauntlet/Blueprints/AI/AIController_Boss0.Start` _asaicontroller_boss_0)))))

(event `/Game/Gauntlet/Blueprints/AI/Spawn/PlayerTriggerable.ResetTriggerability`
  (goto _label :!via `Reset`))

(event `self.ReceiveActorEndOverlap`
  (params (OtherActor :type "Actor Object Reference")))

(event `/Game/Gauntlet/Blueprints/AI/Shooting.ShootAt`
  (params (Target :type "Actor Object Reference"))
  (`/Game/Gauntlet/Blueprints/AI/Shooting.ShootAtLocation` (`self.K2_GetActorLocation` Target)))

(event `/Game/Gauntlet/Blueprints/AI/Shooting.ShootAtLocation`
  (params (Target :type "Vector Structure"))
  (set `self.Shooting` true)
  (`|SpawnActorFromClass` "/Game/Gauntlet/Blueprints/AI/Projectile_Meteor.Projectile_Meteor_C" (`KismetMathLibrary.Conv_VectorToTransform` (+ Target (0.0 0.0 300.0))) false self)
  (set `self.Shooting` false))

(event `/Game/Gauntlet/Blueprints/AI/Spawning.Spawn`
  (set `self.Spawning` true)
  (bind _returnvalue (`|SpawnActorFromClass` "/Game/Gauntlet/Blueprints/AI/AICharacter_Melee.AICharacter_Melee_C" (`KismetMathLibrary.MakeTransform` (+ (.location (`self.GetTransform`)) (256.0 0.0 126.0)) (.rotation (`self.GetTransform`)))))
  (`KismetArrayLibrary.Array_Add` (`self.Spawned`) _returnvalue)
  (`KismetSystemLibrary.Delay` 0.3)
  (set `self.Spawning` false))

(event `/Game/Gauntlet/Blueprints/AI/Invulnerable.BeginInvulnerable`
  (set `self.Invulnerable` true))

(event `/Game/Gauntlet/Blueprints/AI/Invulnerable.StopInvulnerable`
  (set `self.Invulnerable` false))

(fn `GetHealth`
  (returns (Health :type "Float (double-precision)"))
  (return (`self.Health`)))

(fn `GetMaxHealth`
  (returns (MaxHealth :type "Float (double-precision)"))
  (return (`self.MaxHealth`)))

(fn `ShootFinished`
  (returns (Finished :type Boolean))
  (return (not (`self.Shooting`))))

(fn `SpawnFinished`
  (returns (Finished :type Boolean))
  (return (not (`self.Spawning`))))

(fn `UserConstructionScript`)