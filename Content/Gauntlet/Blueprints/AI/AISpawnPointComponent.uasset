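; AI spawn point component that spawns one random actor from its Types class list at the owning actor's location.
; Its Spawn event does nothing when the list is empty, otherwise it picks a random index and spawns that class with the owner's transform.
; The component has no active Tick or BeginPlay logic, so spawning happens only when Spawn is called.
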(event `self.ReceiveTick`
  (params (DeltaSeconds :type "Float (single-precision)")))

(event `self.ReceiveBeginPlay`)

(event `self.Spawn`
  (bind _types (`self.Types`))
  (if (> (`KismetArrayLibrary.Array_Length` (`self.Types`)) 0)
    (`|SpawnActorFromClass` (`KismetArrayLibrary.Array_Get` _types (`KismetMathLibrary.RandomIntegerInRange` 0 (`KismetArrayLibrary.Array_LastIndex` _types))) (`Actor.GetTransform` (`self.GetOwner`)))))