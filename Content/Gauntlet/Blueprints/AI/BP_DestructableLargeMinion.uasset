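; BP_DestructableLargeMinion is a destructible stand-in for a large minion that fades out through its material as soon as it spawns, apparently as a death effect.
; The construction script creates a dynamic instance of the ShockRock character material.
; BeginPlay applies that instance to every material slot on the Destructible component, then plays a timeline that drives its DeathScalar parameter from the DeathFade track.
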(event `self.ReceiveBeginPlay`
  (bind _destructible (`self.Destructible`))
  (for (_ _array_index) (`MeshComponent.GetMaterials` _destructible)
    (`PrimitiveComponent.SetMaterial` _destructible _array_index (`self.MID`)))
  (bind (_direction _deathfade) (`Timeline|Timeline_0` :!via `PlayFromStart`)
    (:`Update`
      (`MaterialInstanceDynamic.SetScalarParameterValue` (`self.MID`) "DeathScalar" _deathfade))))

(event `self.ReceiveActorBeginOverlap`
  (params (OtherActor :type "Actor Object Reference")))

(event `self.ReceiveTick`
  (params (DeltaSeconds :type "Float (single-precision)")))

(fn `UserConstructionScript`
  (bind _returnvalue (`KismetMaterialLibrary.CreateDynamicMaterialInstance` "/Game/Gauntlet/Materials/Ma_Char_ShockRock.Ma_Char_ShockRock"))
  (set `self.MID` _returnvalue))