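; Shockwave projectile for AI attacks that hugs the ground and damages actors it touches.
; Each Tick, a vertical object trace against WorldStatic finds the floor and snaps the actor to a fixed height above it, without sweeping.
; Sphere overlaps apply a small fixed damage to any actor except the Instigator, crediting the instigator's controller, and the projectile is not destroyed on hit.
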(event `self.ReceiveBeginPlay`)

(event `self.ReceiveActorBeginOverlap`
  (params (OtherActor :type "Actor Object Reference")))

(event `self.ReceiveTick`
  (params (DeltaSeconds :type "Float (single-precision)"))
  (bind _returnvalue (`self.K2_GetActorLocation`))
  (bind (_outhit _returnvalue_2) (`KismetSystemLibrary.LineTraceSingleForObjects` (+ _returnvalue (0.0 0.0 200.0)) (+ _returnvalue (0.0 0.0 -200.0)) (`|MakeArray` "ObjectTypeQuery1" :!type "EObjectTypeQuery Enum")))
  (if _returnvalue_2
    (`self.K2_SetActorLocation` (+ (`.Location` (`GameplayStatics.BreakHitResult` _outhit)) (0.0 0.0 100.0)))))

(event `self.Sphere.OnComponentBeginOverlap`
  (params (OtherActor :type "Actor Object Reference") (OtherComp :type "PrimitiveComponent Object Reference") (OtherBodyIndex :type Integer) (bFromSweep :type Boolean) (SweepResult :type "HitResult Structure (by ref)"))
  (if (!= OtherActor (`self.Instigator`))
    (`GameplayStatics.ApplyDamage` OtherActor 3.0 (`self.GetInstigatorController`) self)))

(fn `UserConstructionScript`)