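; Function library for an AutoCurve struct, which samples a float curve against game time without a timeline.
; Start records the game time and sets the Playing flag, while Stop and Resume only toggle that flag.
; GetCurveValue ignores Playing and evaluates the curve at start time minus current time, so the sampled time runs negative after Start.
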(fn `GetCurveValue`
  (params (AutoCurve :type "/Game/Gauntlet/Blueprints/AutoCurve Structure"))
  (returns (Value :type "Float (double-precision)"))
  (bind (_curve _timestarted) (break `/Game/Gauntlet/Blueprints/AutoCurve` AutoCurve))
  (return (`CurveFloat.GetFloatValue` _curve (- _timestarted (`KismetSystemLibrary.GetGameTimeInSeconds` null)))))

(fn `Resume`
  (params (`Auto Curve` :type "/Game/Gauntlet/Blueprints/AutoCurve Structure"))
  (setmembers `/Game/Gauntlet/Blueprints/AutoCurve` :`StructRef` `Auto Curve` :`Playing` true))

(fn `Start`
  (params (`Auto Curve` :type "/Game/Gauntlet/Blueprints/AutoCurve Structure"))
  (setmembers `/Game/Gauntlet/Blueprints/AutoCurve` :`StructRef` `Auto Curve` :`TimeStarted` (`KismetSystemLibrary.GetGameTimeInSeconds` null) :`Playing` true))

(fn `Stop`
  (params (`Auto Curve` :type "/Game/Gauntlet/Blueprints/AutoCurve Structure"))
  (setmembers `/Game/Gauntlet/Blueprints/AutoCurve` :`StructRef` `Auto Curve` :`Playing` false))