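; Camera control trigger volume that signals the player character to adjust its camera, chiefly zoom, while inside an area.
; On entry, it packs its zoom, lerp and reset-on-exit settings with the player's current boom arm length into a CameraPointData struct and passes it to the character.
; On exit, it notifies the character, which handles the camera change itself.
; Only overlaps from the player's capsule component count.
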(event `self.TriggerArea.OnComponentBeginOverlap`
  (params (OtherActor :type "Actor Object Reference") (OtherComp :type "PrimitiveComponent Object Reference") (OtherBodyIndex :type Integer) (bFromSweep :type Boolean) (SweepResult :type "HitResult Structure (by ref)"))
  (bind _asplayer_character (cast `/Game/ThirdPerson/Blueprints/PlayerCharacter` OtherActor))
  (bind _information (`self.CompileCameraPointData` _asplayer_character))
  (if (== (`Character.CapsuleComponent` _asplayer_character) OtherComp)
    (`/Game/ThirdPerson/Blueprints/PlayerCharacter.OnEnterCameraPoint` _asplayer_character _information)))

(event `self.TriggerArea.OnComponentEndOverlap`
  (params (OtherActor :type "Actor Object Reference") (OtherComp :type "PrimitiveComponent Object Reference") (OtherBodyIndex :type Integer))
  (bind _asplayer_character (cast `/Game/ThirdPerson/Blueprints/PlayerCharacter` OtherActor))
  (if (== (`Character.CapsuleComponent` _asplayer_character) OtherComp)
    (`/Game/ThirdPerson/Blueprints/PlayerCharacter.OnExitCameraPoint` _asplayer_character)))

(fn `CompileCameraPointData`
  (params (Player :type "/Game/ThirdPerson/Blueprints/PlayerCharacter Object Reference"))
  (returns (Information :type "/Game/Gauntlet/Blueprints/CameraPointData Structure"))
  (return (make `/Game/Gauntlet/Blueprints/CameraPointData` (`self.ZoomCamera`) (`self.ResetAfterExit`) (`self.TargetCameraLength`) (`SpringArmComponent.TargetArmLength` (`GauntletCharacter.CameraBoom` Player)) (`self.LerpEnterZoomFactor`) (`self.LerpExitZoomFactor`))))

(fn `UserConstructionScript`)