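; ComboText is an effect actor that moves like a tossed popup, presumably for combo text.
; BeginPlay picks a random direction within a cone around world up.
; Each Tick offsets the actor along that direction at BounceSpeed without sweeping, while lerping the direction toward straight down by delta time, producing a rise-then-fall arc without physics.
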(event `self.ReceiveBeginPlay`
  (set `self.Dir` (+ (`KismetMathLibrary.RandomUnitVectorInCone` (0.0 0.0 1.0) 1.0) (0.0 0.0 0.0))))

(event `self.ReceiveActorBeginOverlap`
  (params (OtherActor :type "Actor Object Reference")))

(event `self.ReceiveTick`
  (params (DeltaSeconds :type "Float (single-precision)"))
  (`self.K2_AddActorWorldOffset` (* (`self.Dir`) (* DeltaSeconds (`self.Bounce Speed`))))
  (set `self.Dir` (`KismetMathLibrary.VLerp` (`self.Dir`) (`KismetMathLibrary.MakeVector` 0.0 0.0 -1.0) DeltaSeconds)))

(fn `UserConstructionScript`)