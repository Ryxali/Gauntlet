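; Game mode for Gauntlet that runs the player death and respawn cycle and spawns money pickups.
; Death opens the HUD perk menu; respawn replaces the pawn at the first PlayerStart, resets PlayerTriggerable actors and hides the menu.
; DropMoney passes randomized gold through BuffManager's "Money" value, with a test drop after BeginPlay.
; DropPerk spawns a zero-gold MoneyPickup, and OnEnemyDeath is empty.
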(event Custom|On%20Respawn
  (params (Player :type Player%20Controller%20Object%20Reference))
  (CallFunction|Spawn Player)
  (bind _outactors (Actor|GetAllActorswithInterface "/Game/Gauntlet/Blueprints/AI/Spawn/PlayerTriggerable.PlayerTriggerable_C"))
  (Class|PlayerTriggerable|ResetTriggerability(Message) _outactors)
  (bind _ashudgame (Utilities|Casting|CastToHUDGame (HUD|GetHUD Player)))
  (Default|HidePerkMenu _ashudgame))

(event Custom|OnEnemyDeath
  (params (DeathLocation :type Vector)))

(event Custom|On%20Player%20Death
  (params (Player :type Player%20Controller%20Object%20Reference))
  (bind _ashudgame (Utilities|Casting|CastToHUDGame (HUD|GetHUD Player)))
  (Default|ShowPerkMenu _ashudgame))

(event Custom|DropPerk
  (params (Position :type Vector))
  (Game|SpawnActorfromClass "/Game/Gauntlet/Blueprints/Perks/MoneyPickup.MoneyPickup_C" (Math|Conversions|ToTransform(Vector) Position) false 0 0 0))

(event EventBeginPlay
  (bind _returnvalue (Game|GetPlayerCharacter 0))
  (Class|BuffManagerComponent|AddValue (Variables|Default|GetBuffManager) "Money" 1.0 (Utilities|Array|MakeArray "GOLD_DROP_QUANTITY"))
  (Utilities|FlowControl|Delay 2.0)
  (CallFunction|DropMoney (+ (Transformation|GetActorLocation _returnvalue) (* (Transformation|GetActorForwardVector _returnvalue) 2e+02))))

(event EventTick
  (params (DeltaSeconds :type Float%20%28single-precision%29)))

(fn ConstructionScript)

(fn Spawn
  (params (Player :type Player%20Controller%20Object%20Reference))
  (bind _returnvalue (Pawn|GetControlledPawn Player))
  (Utilities|IsValid _returnvalue
    (:Is%20Valid
      (Actor|DestroyActor _returnvalue))
    (:Is%20Not%20Valid
      _))
  (bind _outactors (Actor|GetAllActorsOfClass "/Script/Engine.PlayerStart"))
  (if (> (Utilities|Array|Length _outactors) 0)
    (bind _returnvalue_2 (Game|SpawnActorfromClass (Variables|Default|GetDefaultPawnClass) (Math|Transform|MakeTransform (.Location (Math|Transform|BreakTransform (Transformation|GetActorTransform (Utilities|Array|Get(acopy) _outactors)))) (.Rotation (Math|Transform|BreakTransform (Transformation|GetActorTransform (Utilities|Array|Get(acopy) _outactors)))) "1,1.000000,1") true 0 0))
    (Pawn|Possess (Game|GetPlayerController 0) _returnvalue_2)
    (else
      (Development|PrintString "ERR no spawn points!"))))

(fn DropMoney
  (params (Location :type Vector))
  (bind _buffmanager (Variables|Default|GetBuffManager))
  (bind _golddropbase (Variables|MoneyPickup|GetGoldDropBase))
  (bind _golddropdeviation (Variables|MoneyPickup|GetGoldDropDeviation))
  (bind _returnvalue (Math|Random|RandomIntegerinRange 0 _golddropdeviation))
  (bind _returnvalue_2 (+ _golddropbase _returnvalue))
  (bind _returnvalue_3 (Math|Conversions|ToFloat(Integer) _returnvalue_2))
  (Development|PrintString (Utilities|String|ToString(Float) _returnvalue_3))
  (bind _output_get (LocalVariables|SetMoney _returnvalue_3))
  (Class|BuffManagerComponent|SetValue _buffmanager "Money" _output_get)
  (Development|PrintString "MONIES")
  (Game|SpawnActorfromClass "/Game/Gauntlet/Blueprints/Perks/MoneyPickup.MoneyPickup_C" (Math|Transform|MakeTransform Location) false 0 (Math|Float|Truncate (Class|BuffManagerComponent|GetValue _buffmanager "Money")) 0))