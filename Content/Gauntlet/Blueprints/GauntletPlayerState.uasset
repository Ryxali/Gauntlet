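; GauntletPlayerState is the player state that tracks gold and hit combos and grants a shielding perk at BeginPlay.
; TickCombo increments the count held in PerkManager and restarts a timeline that feeds remaining time to the HUD and resets the combo when finished.
; An EndComboStreak macro uses a DoOnce, re-armed on each hit, to gate that reset.
; Combo and gold changes are pushed directly to player 0's HUD.
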(event `self.ReceiveTick`
  (params (DeltaSeconds :type "Float (single-precision)")))

(event `self.ReceiveBeginPlay`
  (`PerkManagerComponent.AddPerk` (`self.PerkManager`) "/Game/Gauntlet/Blueprints/Perks/Perk_Shielding.Perk_Shielding_C"))

(event `Run Combo Reset Timer`
  (bind (_direction _timeremainingperc) (`Timeline|ComboTimeout` :!via `PlayFromStart`)
    (:`Update`
      (message `/Game/Gauntlet/Blueprints/HUD/PlayerObserverInterface.AlertNewTimeRemainingCombo` (`PlayerController.GetHUD` (`GameplayStatics.GetPlayerController` 0)) _timeremainingperc))
    (:`Finished`
      (`self.ResetCombo`))))

(fn `AddGold`
  (params (AddedGold :type Integer))
  (bind _output_get (set `self.Money` (+ AddedGold (`self.Money`))))
  (message `/Game/Gauntlet/Blueprints/HUD/PlayerObserverInterface.AlertNewGold` (`PlayerController.GetHUD` (`GameplayStatics.GetPlayerController` 0)) _output_get))

(fn `GetComboCount`
  (returns (`Combo Count` :type Integer))
  (return (`PerkManagerComponent.GetComboCount` (`self.PerkManager`))))

(fn `ResetCombo`
  (`|ExecutionSequence`
    (:`then_0`
      (goto _label :!via `Reset`))
    (:`then_1`
      (`self.EndComboStreak` :!label _label
        (:` `
          (message `/Game/Gauntlet/Blueprints/HUD/PlayerObserverInterface.AlertNewCombo` (`PlayerController.GetHUD` (`GameplayStatics.GetPlayerController` 0)) (`self.GetComboCount`)))))))

(fn `TickCombo`
  (params (EnemyHit :type "Actor Object Reference"))
  (`PerkManagerComponent.IncrementCombo` (`self.PerkManager`) EnemyHit)
  (`|ExecutionSequence`
    (:`then_0`
      (`self.EndComboStreak` :!via `Reset`
        (:` `
          (`self.Run Combo Reset Timer`))))
    (:`then_1`
      (message `/Game/Gauntlet/Blueprints/HUD/PlayerObserverInterface.AlertNewCombo` (`PlayerController.GetHUD` (`GameplayStatics.GetPlayerController` 0)) (`self.GetComboCount`))
      (`KismetSystemLibrary.PrintString` "dadasdad"))))

(fn `UserConstructionScript`)