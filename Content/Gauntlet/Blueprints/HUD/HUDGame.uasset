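; HUDGame is the game's HUD Blueprint, which shows and hides the perk menu for the owning player.
; ShowPerkMenu creates a PerkMenu widget, stores it in Menu, adds it to the viewport and enables the mouse cursor.
; HidePerkMenu removes the stored widget, if valid, and hides the cursor again.
; BeginPlay, EndPlay and the construction script only call their parent versions.
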(event `self.ReceiveEndPlay`
  (params (EndPlayReason :type "EEndPlayReason Enum" :default "Destroyed"))
  (`parent.ReceiveEndPlay` EndPlayReason))

(event `self.ReceiveBeginPlay`
  (`parent.ReceiveBeginPlay`))

(event `self.ReceiveActorBeginOverlap`
  (params (OtherActor :type "Actor Object Reference")))

(event `self.ReceiveTick`
  (params (DeltaSeconds :type "Float (single-precision)")))

(event `ShowPerkMenu`
  (bind _returnvalue (`|CreateWidget` "/Game/Gauntlet/Blueprints/HUD/PerkMenu.PerkMenu_C" (`self.GetOwningPlayerController`)))
  (bind _output_get (set `self.Menu` _returnvalue))
  (`UserWidget.AddToViewport` _output_get 0)
  (set `PlayerController.bShowMouseCursor` true (`self.GetOwningPlayerController`)))

(event `HidePerkMenu`
  (bind _menu (`self.Menu`)
    (:`then`
      (`Widget.RemoveFromParent` _menu)
      (set `PlayerController.bShowMouseCursor` false (`self.GetOwningPlayerController`)))
    (:`else`)))

(fn `UserConstructionScript`
  (`parent.UserConstructionScript`))