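; Menu HUD that shows the game's menus and manages forward and back navigation between them.
; It creates MenuBase_BP on BeginPlay and removes the current menu on EndPlay.
; Entering a new menu pushes the current widget's class onto a History stack and swaps in the new widget.
; Going back pops the stack and recreates that menu from its class, doing nothing when History is empty at the root.
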(event `self.ReceiveBeginPlay`
  (`parent.ReceiveBeginPlay`)
  (bind _returnvalue (`|CreateWidget` "/Game/Gauntlet/Blueprints/HUD/Menu/MenuBase_BP.MenuBase_BP_C" (`GameplayStatics.GetPlayerController` 0)))
  (bind _output_get (set `self.CurrentMenu` _returnvalue))
  (`UserWidget.AddToViewport` _output_get (`self.MenuLayer`)))

(event `self.ReceiveActorBeginOverlap`
  (params (OtherActor :type "Actor Object Reference")))

(event `self.ReceiveTick`
  (params (DeltaSeconds :type "Float (single-precision)")))

(event `self.ReceiveEndPlay`
  (params (EndPlayReason :type "EEndPlayReason Enum" :default "Destroyed"))
  (`parent.ReceiveEndPlay` EndPlayReason)
  (`Widget.RemoveFromParent` (`self.CurrentMenu`)))

(fn `EnterNewMenuState`
  (params (StateType :type "UserWidget Class Reference"))
  (`|ExecutionSequence`
    (:`then_0`
      (bind _currentmenu (`self.CurrentMenu`)
        (:`then`
          (`|ExecutionSequence`
            (:`then_0`
              (bind _asuser_widget (castclass `UserWidget` (`GameplayStatics.GetObjectClass` _currentmenu)))
              (`KismetArrayLibrary.Array_Add` (`self.History`) _asuser_widget))
            (:`then_1`
              (`Widget.RemoveFromParent` _currentmenu))))
        (:`else`)))
    (:`then_1`
      (bind _returnvalue (`|CreateWidget` StateType (`GameplayStatics.GetPlayerController` 0)))
      (bind _output_get (set `self.CurrentMenu` _returnvalue))
      (`UserWidget.AddToViewport` _output_get 0))))

(fn `EnterPreviousMenuState`
  (bind _history (`self.History`))
  (bind _returnvalue (`KismetArrayLibrary.Array_LastIndex` _history))
  (if (not (`self.IsMenuAtRoot`))
    (`|ExecutionSequence`
      (:`then_0`
        (bind _currentmenu (`self.CurrentMenu`)
          (:`then`
            (`Widget.RemoveFromParent` _currentmenu))
          (:`else`)))
      (:`then_1`
        (bind _returnvalue_2 (`|CreateWidget` (`KismetArrayLibrary.Array_Get` _history _returnvalue) (`GameplayStatics.GetPlayerController` 0)))
        (bind _output_get (set `self.CurrentMenu` _returnvalue_2))
        (`UserWidget.AddToViewport` _output_get 0)
        (`KismetArrayLibrary.Array_Remove` _history _returnvalue)))))

(fn `IsMenuAtRoot`
  (returns (IsRoot :type Boolean))
  (return (== (`KismetArrayLibrary.Array_Length` (`self.History`)) 0)))

(fn `UserConstructionScript`)