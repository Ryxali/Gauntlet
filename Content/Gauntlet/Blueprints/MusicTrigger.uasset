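; MusicTrigger is a box trigger actor that steps up the intensity of the canyon music when the player enters it.
; On overlap with the PlayerCharacter class, it reads the MusicIntensity parameter from the Manager's MusicCanyon and writes it back one higher.
; A HasTriggered flag limits this to a single firing until the Reset event clears it, with debug strings printed along the way.
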(event `self.ReceiveBeginPlay`)

(event `self.ReceiveActorBeginOverlap`
  (params (OtherActor :type "Actor Object Reference")))

(event `self.ReceiveTick`
  (params (DeltaSeconds :type "Float (single-precision)")))

(event `self.Box.OnComponentBeginOverlap`
  (params (OtherActor :type "Actor Object Reference") (OtherComp :type "PrimitiveComponent Object Reference") (OtherBodyIndex :type Integer) (bFromSweep :type Boolean) (SweepResult :type "HitResult Structure (by ref)"))
  (bind _musiccanyon (`/Game/Gauntlet/Blueprints/MusicManager.MusicCanyon` (`self.Manager`)))
  (if (== (`GameplayStatics.GetObjectClass` OtherActor) "/Game/ThirdPerson/Blueprints/PlayerCharacter.PlayerCharacter_C")
    (if (`self.HasTriggered`)
      (`KismetSystemLibrary.PrintString` "HAs already triggered")
      (else
        (`KismetSystemLibrary.PrintString` "Jag hade ingen lätt barndom, när jag frågade mina föräldrar om vi kunde åka till djurparken så sa dem: \"Om de vill ha dig så kommer de och hämtar dig.\"")
        (set `self.HasTriggered` true)
        (bind _returnvalue (`FMODAudioComponent.GetParameter` _musiccanyon "MusicIntensity"))
        (bind _returnvalue_2 (+ _returnvalue 1.0))
        (`FMODAudioComponent.SetParameter` _musiccanyon "MusicIntensity" _returnvalue_2)
        (`KismetSystemLibrary.PrintString` (`KismetStringLibrary.Conv_DoubleToString` _returnvalue_2))))))

(event `/Game/Gauntlet/Blueprints/Interfaces/Resetable.Reset`
  (set `self.HasTriggered` false))

(fn `UserConstructionScript`)