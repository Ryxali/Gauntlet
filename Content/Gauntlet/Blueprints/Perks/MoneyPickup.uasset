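; Pooled money pickup that homes in on the local player and awards gold on contact.
; A magnet sphere sets the target; Tick then moves the pickup forward while rotating toward it, scaling both speeds with a distance-based curve.
; After a cooldown, touching the player's capsule adds gold to GauntletPlayerState and returns the actor to the game mode's MoneyPool.
; InitRandomDirection provides a random upward-cone starting heading for curved homing paths.
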(event OnComponentBeginOverlap(PickupSphere)
  (params (OtherActor :type Actor%20Object%20Reference) (OtherComp :type Primitive%20Component%20Object%20Reference) (OtherBodyIndex :type Integer) (bFromSweep :type Boolean) (SweepResult :type Hit%20Result%20Structure%20%28by%20ref%29))
  (bind _returnvalue (Game|GetPlayerCharacter 0))
  (if (<= (Variables|Default|GetCooldownForPickup) 0.0)
    (if (and (== OtherComp (Variables|/Script/Engine.Character|GetCapsuleComponent _returnvalue)) (== OtherActor _returnvalue))
      (bind _ascharacter (Utilities|Casting|CastToCharacter OtherActor))
      (bind _asgauntlet_player_state (Utilities|Casting|CastToGauntletPlayerState (Variables|/Script/Engine.Pawn|GetPlayerState _ascharacter)))
      (CallFunction|AddMoney _asgauntlet_player_state)
      (bind _asgame_mode_game (Utilities|Casting|CastToGameModeGame (Game|GetGameMode)))
      (Default|ReturnObject (Variables|/Game/Gauntlet/Blueprints/GameModeGame.GameModeGame_C|GetMoneyPool _asgame_mode_game) self))))

(event OnComponentBeginOverlap(MagnetSphere)
  (params (OtherActor :type Actor%20Object%20Reference) (OtherComp :type Primitive%20Component%20Object%20Reference) (OtherBodyIndex :type Integer) (bFromSweep :type Boolean) (SweepResult :type Hit%20Result%20Structure%20%28by%20ref%29))
  (bind _ascharacter (Utilities|Casting|CastToCharacter OtherActor))
  (if (Pawn|IsLocalPlayerController (Pawn|GetController _ascharacter))
    (Variables|Default|SetTarget OtherActor)))

(event EventBeginPlay)

(event Collision|EventActorBeginOverlap
  (params (OtherActor :type Actor%20Object%20Reference)))

(event EventTick
  (params (DeltaSeconds :type Float%20%28single-precision%29))
  (Variables|Default|SetCooldownForPickup (- (Variables|Default|GetCooldownForPickup) DeltaSeconds))
  (bind _target (Variables|Default|GetTarget)
    (:then
      (Transformation|SetActorLocation (+ (Transformation|GetActorLocation) (* (Transformation|GetActorForwardVector) (* (Variables|Default|GetFloatSpeed) DeltaSeconds (CallFunction|GetSpeedFactor)))) false)
      (Transformation|SetActorRotation (Class|KismetMathLibrary|RInterptoConstant (Transformation|GetActorRotation) (Math|Rotator|FindLookatRotation (Transformation|GetActorLocation) (Transformation|GetActorLocation _target)) DeltaSeconds (* (Variables|Default|GetRotSpeed) (CallFunction|GetSpeedFactor)))))
    (:else)))

(fn ConstructionScript)

(fn AddMoney
  (params (NewParam :type Gauntlet%20Player%20State%20Object%20Reference))
  (Default|AddGold NewParam (Variables|Default|GetGoldWorth)))

(fn GetSpeedFactor
  (return (Math|Curves|GetFloatValue (Variables|Default|GetSpeedCurve) (Math|Float|Clamp(Float) (- 1.0 (Class|KismetMathLibrary|InverseLerp 3e+02 6e+02 (Math|Vector|VectorLength (- (Transformation|GetActorLocation (Variables|Default|GetTarget)) (Transformation|GetActorLocation))))) 0.4))))

(fn InitRandomDirection
  (bind _returnvalue (Transformation|GetActorLocation))
  (Transformation|SetActorRotation (Math|Rotator|FindLookatRotation _returnvalue (+ (Class|KismetMathLibrary|RandomUnitVectorinCone "0, 0,1.000000" 1.0) _returnvalue))))