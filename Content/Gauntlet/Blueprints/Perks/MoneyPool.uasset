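; MoneyPool is an object pool of MoneyPickup actors, pre-spawned on BeginPlay and kept hidden with tick and collision off.
; RetriveObject activates the last cached pickup and moves it to the active list, while ReturnObject deactivates it and puts it back.
; Both arrays are resized before filling, so they start with empty slots.
; Retrieval ignores its Worth input and has no empty-cache check.
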(event EventBeginPlay
  (bind _moneycachesize (Variables|Default|GetMoneyCacheSize))
  (Utilities|Array|Resize (Variables|Default|GetMoneyCache) _moneycachesize)
  (Utilities|Array|Resize (Variables|Default|GetActiveMoneyInstances) _moneycachesize)
  (for _index (range 0 (Variables|Default|GetMoneyCacheSize))
    (bind _returnvalue (Game|SpawnActorfromClass "/Game/Gauntlet/Blueprints/Perks/MoneyPickup.MoneyPickup_C" (Math|Transform|MakeTransform "0, 0, 0") false 0 10 0))
    (CallFunction|DeactivateActor _returnvalue)
    (Utilities|Array|Add (Variables|Default|GetMoneyCache) _returnvalue)))

(fn ConstructionScript)

(fn ActivateActor
  (params (Actor :type Money%20Pickup%20Object%20Reference))
  (Actor|Tick|SetActorTickEnabled Actor true)
  (Collision|SetActorEnableCollision Actor true)
  (Rendering|SetActorHiddenInGame Actor false))

(fn DeactivateActor
  (params (Actor :type Money%20Pickup%20Object%20Reference))
  (Rendering|SetActorHiddenInGame Actor true)
  (Actor|Tick|SetActorTickEnabled Actor)
  (Collision|SetActorEnableCollision Actor false))

(fn RetriveObject
  (params (Worth :type Integer))
  (bind _output_get (LocalVariables|SetIndex (- (Utilities|Array|Length (Variables|Default|GetMoneyCache)) 1)))
  (bind _output_get_2 (LocalVariables|SetActor (Utilities|Array|Get(acopy) (Variables|Default|GetMoneyCache) _output_get)))
  (CallFunction|ActivateActor _output_get_2)
  (Utilities|Array|Add (Variables|Default|GetActiveMoneyInstances) (LocalVariables|GetActor))
  (Utilities|Array|RemoveIndex (Variables|Default|GetMoneyCache) (LocalVariables|GetIndex))
  (return (LocalVariables|GetActor)))

(fn ReturnObject
  (params (Instance :type Money%20Pickup%20Object%20Reference))
  (CallFunction|DeactivateActor Instance)
  (Utilities|Array|RemoveItem (Variables|Default|GetActiveMoneyInstances) Instance)
  (Utilities|Array|Add (Variables|Default|GetMoneyCache) Instance))