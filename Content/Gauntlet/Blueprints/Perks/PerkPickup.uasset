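; Perk pickup actor that grants its Perk to the player when touched.
; When the player character overlaps its Sphere, it adds the Perk uniquely to CurrentPerks on GameStateGame, then calls ApplyPerks on the ThirdPersonCharacter.
; A Sequence then destroys the pickup, even if either cast fails.
; A leftover debug string prints on each pickup.
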(event `self.ReceiveBeginPlay`)

(event `self.ReceiveActorBeginOverlap`
  (params (OtherActor :type "Actor Object Reference")))

(event `self.ReceiveTick`
  (params (DeltaSeconds :type "Float (single-precision)")))

(event `self.Sphere.OnComponentBeginOverlap`
  (params (OtherActor :type "Actor Object Reference") (OtherComp :type "PrimitiveComponent Object Reference") (OtherBodyIndex :type Integer) (bFromSweep :type Boolean) (SweepResult :type "HitResult Structure (by ref)"))
  (if (== OtherActor (`GameplayStatics.GetPlayerCharacter` null))
    (`|ExecutionSequence`
      (:`then_0`
        (`KismetSystemLibrary.PrintString` null "BLACKADDER")
        (bind _asgame_state_game (cast `/Game/Gauntlet/Blueprints/GameStateGame` (`GameplayStatics.GetGameState` null)))
        (`KismetArrayLibrary.Array_AddUnique` (`/Game/Gauntlet/Blueprints/GameStateGame.CurrentPerks` _asgame_state_game) (`self.Perk`))
        (bind _asthird_person_character (cast `/Game/ThirdPerson/Blueprints/ThirdPersonCharacter` (`GameplayStatics.GetPlayerCharacter` 0)))
        (`/Game/ThirdPerson/Blueprints/ThirdPersonCharacter.ApplyPerks` _asthird_person_character))
      (:`then_1`
        (`self.K2_DestroyActor`)))))

(fn `UserConstructionScript`)