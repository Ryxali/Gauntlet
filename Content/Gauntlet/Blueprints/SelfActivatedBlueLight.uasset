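; A Blueprint light prop whose emissive glow reacts to the player character's capsule entering and leaving its collision volume.
; The construction script creates a dynamic material instance and gathers static mesh components, which receive that material on BeginPlay.
; Entering plays ImpactTimeline to drive the glow parameter and records its current value.
; Leaving stops that timeline and runs a second one that blends between a dim level and the recorded value.
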(event `self.ReceiveBeginPlay`
  (`PrimitiveComponent.SetMaterial` (`self.Meshes`) 0 (`self.MID`)))

(event `self.ReceiveActorBeginOverlap`
  (params (OtherActor :type "Actor Object Reference")))

(event `self.ReceiveTick`
  (params (DeltaSeconds :type "Float (single-precision)")))

(event `self.Collision.OnComponentBeginOverlap`
  (params (OtherActor :type "Actor Object Reference") (OtherComp :type "PrimitiveComponent Object Reference") (OtherBodyIndex :type Integer) (bFromSweep :type Boolean) (SweepResult :type "HitResult Structure (by ref)"))
  (bind _returnvalue (`GameplayStatics.GetPlayerCharacter` 0))
  (if (and (== OtherActor _returnvalue) (== OtherComp (`Character.CapsuleComponent` _returnvalue)))
    (`|ExecutionSequence`
      (:`then_0`
        (bind (_direction _newtrack_3) (`Timeline|Timeline_0` :!via `Stop` :!label _label)
          (:`Update`
            (`MaterialInstanceDynamic.SetScalarParameterValue` (`self.MID`) "EmissiveGlowiness" (`KismetMathLibrary.Lerp` 0.1 (`self.current glow value`) _newtrack_3)))))
      (:`then_1`
        (bind (_direction_2 _scalar) (`Timeline|ImpactTimeline` :`NewTime` 0.554 :!via `PlayFromStart` :!label _label_2)
          (:`Update`
            (bind _output_get (set `self.current glow value` _scalar))
            (`MaterialInstanceDynamic.SetScalarParameterValue` (`self.MID`) "EmissiveGlowiness" _output_get)))))))

(event `self.Collision.OnComponentEndOverlap`
  (params (OtherActor :type "Actor Object Reference") (OtherComp :type "PrimitiveComponent Object Reference") (OtherBodyIndex :type Integer))
  (bind _returnvalue (`GameplayStatics.GetPlayerCharacter` 0))
  (if (and (== OtherActor _returnvalue) (== OtherComp (`Character.CapsuleComponent` _returnvalue)))
    (`|ExecutionSequence`
      (:`then_0`
        (goto _label_2 :!via `Stop`))
      (:`then_1`
        (goto _label :!via `PlayFromStart`)))))

(fn `UserConstructionScript`
  (bind _returnvalue (`KismetMaterialLibrary.CreateDynamicMaterialInstance` "/Game/Gauntlet/Materials/Glow.Glow"))
  (set `self.MID` _returnvalue)
  (set `self.Meshes` (`self.K2_GetComponentsByClass` "/Script/Engine.StaticMeshComponent")))