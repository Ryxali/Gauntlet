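; SuperMysteriousPillar is an actor whose emissive glow animates when the player character's capsule enters or leaves its Collision volume.
; The construction script creates one dynamic Glow material instance and assigns it to static meshes tagged "Glows".
; On entry, one timeline drives EmissiveGlowiness and records its current value.
; On exit, a second timeline lerps between a dim baseline and that value, so interrupted transitions use the reached brightness.
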(event `self.Collision.OnComponentBeginOverlap`
  (params (OtherActor :type "Actor Object Reference") (OtherComp :type "PrimitiveComponent Object Reference") (OtherBodyIndex :type Integer) (bFromSweep :type Boolean) (SweepResult :type "HitResult Structure (by ref)"))
  (bind _returnvalue (`GameplayStatics.GetPlayerCharacter` 0))
  (if (and (== OtherActor _returnvalue) (== OtherComp (`Character.CapsuleComponent` _returnvalue)))
    (`|ExecutionSequence`
      (:`then_0`
        (bind (_direction _newtrack_3) (`Timeline|Timeline_1` :!via `Stop` :!label _label)
          (:`Update`
            (`MaterialInstanceDynamic.SetScalarParameterValue` (`self.MID`) "EmissiveGlowiness" (`KismetMathLibrary.Lerp` 0.1 (`self.current glow value`) _newtrack_3)))))
      (:`then_1`
        (bind (_direction_2 _scalar) (`Timeline|Timeline_0` :`NewTime` 0.554 :!via `PlayFromStart` :!label _label_2)
          (:`Update`
            (bind _output_get (set `self.current glow value` _scalar))
            (`MaterialInstanceDynamic.SetScalarParameterValue` (`self.MID`) "EmissiveGlowiness" _output_get)))))))

(event `self.Collision.OnComponentEndOverlap`
  (params (OtherActor :type "Actor Object Reference") (OtherComp :type "PrimitiveComponent Object Reference") (OtherBodyIndex :type Integer))
  (bind _returnvalue (`GameplayStatics.GetPlayerCharacter` 0))
  (if (and (== OtherActor _returnvalue) (== OtherComp (`Character.CapsuleComponent` _returnvalue)))
    (`|ExecutionSequence`
      (:`then_0`
        (goto _label_2 :!via `Stop`))
      (:`then_1`
        (goto _label :!via `PlayFromStart`)))))

(event `self.ReceiveBeginPlay`)

(event `self.ReceiveActorBeginOverlap`
  (params (OtherActor :type "Actor Object Reference")))

(event `self.ReceiveTick`
  (params (DeltaSeconds :type "Float (single-precision)")))

(fn `UserConstructionScript`
  (bind _returnvalue (`KismetMaterialLibrary.CreateDynamicMaterialInstance` "/Game/Gauntlet/Materials/Glow.Glow"))
  (bind _output_get (set `self.MID` _returnvalue))
  (bind _output_get_2 (set `self.Meshes` (`self.GetComponentsByTag` "/Script/Engine.StaticMeshComponent" "Glows")))
  (`PrimitiveComponent.SetMaterial` _output_get_2 0 _output_get))