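; Utils is a Blueprint library of small math helpers for rotations and angles in the Gauntlet game.
; FindLookAtRotation2D builds a yaw-only rotation from a start toward a target by flattening the direction onto the XY plane with world Z as up.
; Angle and Angle2D return degrees between two directions via dot product and arccosine; only the 2D version drops Z and normalizes its inputs first.
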(fn `Angle`
  (params (Dir1 :type "Vector Structure") (Dir2 :type "Vector Structure"))
  (returns (Angle :type "Float (double-precision)"))
  (return (`KismetMathLibrary.DegAcos` (`KismetMathLibrary.Dot_VectorVector` Dir1 Dir2))))

(fn `Angle2D`
  (params (Dir1 :type "Vector Structure") (Dir2 :type "Vector Structure"))
  (returns (Angle :type "Float (double-precision)"))
  (return (`KismetMathLibrary.DegAcos` (`KismetMathLibrary.DotProduct2D` (`KismetMathLibrary.Normal2D` (`KismetMathLibrary.MakeVector2D` (.x Dir1) (.y Dir1))) (`KismetMathLibrary.Normal2D` (`KismetMathLibrary.MakeVector2D` (.x Dir2) (.y Dir2)))))))

(fn `FindLookAtRotation 2D`
  (params (Start :type "Vector Structure") (Target :type "Vector Structure"))
  (returns (`Return Value` :type "Rotator Structure"))
  (return (`KismetMathLibrary.MakeRotFromXZ` (`KismetMathLibrary.NegateVector` (`KismetMathLibrary.Normal` (`KismetMathLibrary.MakeVector` (.x (- Start Target)) (.y (- Start Target))))) (`KismetMathLibrary.MakeVector` 0.0 0.0 1.0))))